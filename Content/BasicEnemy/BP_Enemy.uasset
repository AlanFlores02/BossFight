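; BP_Enemy is a basic enemy that hops on spotting a pawn, then chases and self-destructs.
; A State variable gates PawnSensing: the first sighting triggers a timed jump phase, after which sightings drive AIMoveTo toward the seen pawn.
; Movement mode changes during the jump phase call Jump again.
; Reaching the target or running out of health shares one path that spawns an explosion effect and destroys the actor.
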(event OnSeePawn(PawnSensing)
  (params (Pawn :type Pawn%20Object%20Reference))
  (switch int (Variables|Default|GetState)
    (:0
      (Variables|Default|SetState 2)
      (Variables|Default|SetJumping true)
      (Character|Jump)
      (Utilities|FlowControl|Delay 1.0)
      (Variables|Default|SetJumping false)
      (Utilities|FlowControl|Delay 0.2)
      (Variables|Default|SetState 1))
    (:1
      (AI|AIMoveTo self "0, 0, 0" Pawn 5e+01 false
        (:OnSuccess
          ;[1 1 1] Self Destruct
          (Game|SpawnActorfromClass "/Game/StarterContent/Blueprints/Blueprint_Effect_Explosion.Blueprint_Effect_Explosion_C" (Transformation|GetActorTransform) "AlwaysSpawn" 0 0)
          (Actor|DestroyActor))))))

(event EventOnMovementModeChanged
  (params (PrevMovementMode :type EMovementMode%20Enum :default "MOVE_None") (NewMovementMode :type EMovementMode%20Enum :default "MOVE_None") (PrevCustomMode :type Byte :default 0) (NewCustomMode :type Byte :default 0))
  (if (Variables|Default|GetJumping)
    (Character|Jump)))

(event Game|Damage|EventAnyDamage
  (params (Damage :type Float%20%28single-precision%29) (DamageType :type Damage%20Type%20Object%20Reference) (InstigatedBy :type Controller%20Object%20Reference) (DamageCauser :type Actor%20Object%20Reference))
  (bind _output_get (Variables|Default|SetHealth (- (Variables|Default|GetHealth) Damage)))
  (if (<= _output_get 0.0)
    ;[1 1 1] Self Destruct
    (Game|SpawnActorfromClass "/Game/StarterContent/Blueprints/Blueprint_Effect_Explosion.Blueprint_Effect_Explosion_C" (Transformation|GetActorTransform) "AlwaysSpawn" 0 0)
    (Actor|DestroyActor)))

(fn ConstructionScript)