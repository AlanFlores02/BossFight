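; Boss enemy missile projectile that flies along its local Z axis and explodes on impact.
; Each Tick it moves by a swept offset at MoveSpeed, spawning an explosion effect and destroying itself on a blocking hit.
; Otherwise it blends its current rotation toward zero rotation, with an alpha that grows over RotateTime.
; SetVariables sets the speed and rotation time.
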(event EventTick
  (params (DeltaSeconds :type Float%20%28single-precision%29))
  ;[1 1 1] Move
  (bind _sweephitresult (Transformation|AddLocalOffset (Variables|Default|GetCollider) (Math|Vector|MakeVector 0.0 0.0 (* DeltaSeconds (Variables|Default|GetMove%20Speed))) true false))
  ;[1 1 1] On Collision
  (if (.bBlockingHit (Collision|BreakHitResult _sweephitresult))
    (Game|SpawnActorfromClass "/Game/StarterContent/Blueprints/Blueprint_Effect_Explosion.Blueprint_Effect_Explosion_C" (Math|Conversions|ToTransform(Vector) (.Location (Collision|BreakHitResult _sweephitresult))) "AlwaysSpawn" 0 0)
    (Actor|DestroyActor)
    (else
      (bind _output_get (Variables|Default|SetRotate%20Progress (Math|Float|Clamp(Float) (+ (/ DeltaSeconds (Variables|Default|GetRotate%20Time)) (Variables|Default|GetRotate%20Progress)))))
      (Transformation|SetActorRotation (Math|Rotator|Lerp(Rotator) (Transformation|GetActorRotation) "0, 0, 0" _output_get true)))))

(fn ConstructionScript)

(fn SetVariables
  (params (New%20Speed :type Float%20%28double-precision%29) (New%20Rotation :type Float%20%28double-precision%29))
  (Variables|Default|SetMove%20Speed New%20Speed)
  (Variables|Default|SetRotate%20Time New%20Rotation))