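; Boss robot that turns toward the player and fights within a square area around the world origin, with its death triggering the win screen.
; A one-second timer fires missiles from alternating cannons while draining HEAT.
; A hand-coded decision tree on Tick spends low HEAT on a close-range smash or a long-range eye laser, each restoring HEAT and starting a cooldown.
; A Gate enables the laser's lagged aim and line-trace damage.
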(event Custom|Close%20Laser
  (bind _laser_impact (Variables|Default|GetLaser%20Impact))
  (bind _laser (Variables|Default|GetLaser))
  (bind _returnvalue (Transformation|GetWorldLocation _laser))
  ;[1 1 1] VFX Laser Impact
  (Utilities|FlowControl|Gate true) ; enters at Close
)

(event Custom|Open%20Laser
  (bind _laser_impact (Variables|Default|GetLaser%20Impact))
  (bind _laser (Variables|Default|GetLaser))
  (bind _returnvalue (Transformation|GetWorldLocation _laser))
  ;[1 1 1] VFX Laser Impact
  (Utilities|FlowControl|Gate true) ; enters at Open
)

(event Custom|Behavior%20Tree
  (bind _laser_prepare (Variables|Default|GetLaser%20Prepare))
  (bind _heat (Variables|Default|GetHEAT))
  ;[1 1 1] Behavior Tree
  (if (Variables|Default|GetCan%20Attack%20?)
    (if (<= _heat 0)
      (if (<= (Variables|Default|GetSmash%20Contemplation) 0.0)
        (CallFunction|AttackActions 4 1.0) ; Smash!
        (Animation|Montage|PlayMontage (Variables|Default|GetMesh) 0 1.0 0.0 "Start"
          (:then
            (Utilities|FlowControl|Delay 0.15)
            (Game|SpawnActorfromClass "/Game/BossEnemy/VFX/BP_Golpe.BP_Golpe_C" (Math|Transform|MakeTransform (Transformation|GetWorldLocation (Variables|Default|GetSmash%20Area)) "0, 0, 0" "1.000000,1.000000,1.000000") "AlwaysSpawn" 0 0)))
        (elif (<= _heat -5)
          (bind _distance (CallFunction|GetDistancefromPlayer (Variables|Default|GetDefaultSceneRoot)))
          (if (> _distance (Variables|Default|GetMelee%20Range))
            (CallFunction|AttackActions 10 7.0) ; Super Laser
            (Transformation|SetActorLocation _laser_prepare (Transformation|GetWorldLocation (Variables|Default|GetLaser)) false false)
            (Utilities|FlowControl|Delay 2.0)
            (Transformation|SetActorLocation _laser_prepare "0.000000,0.000000,-200.000000" false false)
            (CallFunction|OpenLaser)
            (Components|Activation|Activate (Variables|Default|GetLaser) false)
            (Utilities|FlowControl|Delay 5.0)
            (CallFunction|CloseLaser)
            (Components|Activation|Deactivate (Variables|Default|GetLaser))))))))

(event Custom|Release%20HEAT
  (bind _returnvalue (Game|Player|GetPlayerPawn 0))
  (bind _returnvalue_2 (Transformation|GetActorLocation _returnvalue))
  (if (and (Variables|Default|GetCan%20Attack%20?) (Math|Boolean|ANDBoolean (Utilities|IsValid _returnvalue) (< (Math|Float|Absolute(Float) (.x _returnvalue_2)) 1.5e+03) (< (Math|Float|Absolute(Float) (.y _returnvalue_2)) 1.5e+03)))
    (Math|Integer|DecrementInt (Variables|Default|GetHEAT)
      (:%20%20
        (CallFunction|FireMissile)))))

(event Custom|Attack%20Actions
  (params (HEAT%20Gen :type Integer) (Cooldown :type Float%20%28double-precision%29))
  (Variables|Default|SetHEAT HEAT%20Gen)
  (Variables|Default|SetCan%20Attack%20? false)
  (Variables|Default|SetRotation%20Speed 0.25)
  (Utilities|FlowControl|Delay Cooldown)
  (Variables|Default|SetRotation%20Speed 2.0)
  (Variables|Default|SetCan%20Attack%20? true))

(event EventBeginPlay
  (Utilities|Time|SetTimerbyEvent (delegate Custom|Release%20HEAT) 1.0 true)
  (bind _returnvalue (Actor|GetActorOfClass "/Game/BossEnemy/VFX/BP_ImpactParticles.BP_ImpactParticles_C"))
  (Variables|Default|SetLaser%20Impact _returnvalue)
  (bind _returnvalue_2 (Actor|GetActorOfClass "/Game/BossEnemy/VFX/BP_PrepareLaser.BP_PrepareLaser_C"))
  (Variables|Default|SetLaser%20Prepare _returnvalue_2))

(event Game|Damage|EventAnyDamage
  (params (Damage :type Float%20%28single-precision%29) (DamageType :type Damage%20Type%20Object%20Reference) (InstigatedBy :type Controller%20Object%20Reference) (DamageCauser :type Actor%20Object%20Reference))
  (bind _output_get (Variables|Default|SetHealth (Math|Float|Clamp(Float) (- (Variables|Default|GetHealth) Damage) 0.0 1e+02)))
  (bind _asbp_first_person_character (Utilities|Casting|CastToBP_FirstPersonCharacter (Game|Player|GetPlayerPawn 0)))
  (Default|NewEnemyValue (Variables|/Game/FirstPerson/Blueprints/BP_FirstPersonCharacter.BP_FirstPersonCharacter_C|GetHUD _asbp_first_person_character) (/ _output_get 5e+01))
  (if (<= (Math|Float|Clamp(Float) (- (Variables|Default|GetHealth) Damage) 0.0 1e+02) 0.0)
    (Input|DisableInput _asbp_first_person_character (Game|GetPlayerController 0))
    (Game|SpawnActorfromClass "/Game/BossEnemy/VFX/BP_BigBoom.BP_BigBoom_C" (Math|Transform|MakeTransform (Transformation|GetActorLocation) "0, 0, 0" "1.000000,1.000000,1.000000") "Undefined" 0 0)
    (Default|GameOver (Variables|/Game/FirstPerson/Blueprints/BP_FirstPersonCharacter.BP_FirstPersonCharacter_C|GetHUD _asbp_first_person_character) "¡¡¡Ganaste!!!" "(R=0.000000,G=0.800000,B=0.000000,A=0.800000)")
    (Actor|DestroyActor)))

(event EventTick
  (params (DeltaSeconds :type Float%20%28single-precision%29))
  (bind _returnvalue (Game|Player|GetPlayerPawn 0))
  (bind _laser_impact (Variables|Default|GetLaser%20Impact))
  (bind _laser (Variables|Default|GetLaser))
  (bind _returnvalue_2 (Transformation|GetWorldLocation _laser))
  (bind _returnvalue_3 (Transformation|GetActorLocation _returnvalue))
  (if (Math|Boolean|ANDBoolean (Utilities|IsValid _returnvalue) (< (Math|Float|Absolute(Float) (.x _returnvalue_3)) 1.5e+03) (< (Math|Float|Absolute(Float) (.y _returnvalue_3)) 1.5e+03))
    (CallFunction|PrepareSmashAttack DeltaSeconds)
    (CallFunction|BehaviorTree)
    (CallFunction|Rotate DeltaSeconds)
    ;[1 1 1] VFX Laser Impact
    (Utilities|FlowControl|Gate true
      (:Exit
        (CallFunction|RollEyes DeltaSeconds)
        (bind (_outhit _returnvalue_4) (Collision|LineTraceByChannel _returnvalue_2 (+ _returnvalue_2 (Math|Vector|RotateVector "2000.000000,0.000000,0.000000" (Transformation|GetWorldRotation _laser))) "TraceTypeQuery2" false 0 "ForOneFrame"))
        (if _returnvalue_4
          (Game|Damage|ApplyDamage (.HitActor (Collision|BreakHitResult _outhit)) (* DeltaSeconds 1e+01) 0 0)
          (Transformation|SetActorLocation _laser_impact (.Location (Collision|BreakHitResult _outhit)) false false)
          (Utilities|FlowControl|RetriggerableDelay 0.1)
          (Transformation|SetActorLocation _laser_impact "0.000000,0.000000,-200.000000" false false))))))

(fn ConstructionScript
  (bind _mesh (Variables|Default|GetMesh))
  (Transformation|AttachComponentToComponent (Variables|Default|GetL%20Hand%20Collider) _mesh "left_hand" "SnapToTarget" "SnapToTarget" "KeepRelative" true)
  (Transformation|AttachComponentToComponent (Variables|Default|GetR%20Hand%20Collider) _mesh "right_hand" "SnapToTarget" "SnapToTarget" "KeepRelative" true)
  (Transformation|AttachComponentToComponent (Variables|Default|GetLaser) _mesh "eye" "SnapToTarget" "SnapToTarget" "KeepRelative" true))

(fn GetDistancefromPlayer
  (params (Component :type Scene%20Component%20Object%20Reference))
  (return (Math|Vector|Distance(Vector) (Transformation|GetWorldLocation Component) (Transformation|GetActorLocation (Game|Player|GetPlayerPawn 0)))))

(fn FireMissile
  (Variables|Default|SetCannon%20Turn (not (Variables|Default|GetCannon%20Turn))) ; Switch cannon to use each shot
  (bind _returnvalue (Game|SpawnActorfromClass "/Game/BossEnemy/BP_Missile.BP_Missile_C" (Math|Transform|MakeTransform (.location (Transformation|GetSocketTransform (Variables|Default|GetMesh) (select (Variables|Default|GetCannon%20Turn) "right_cannon" "left_cannon") "RTS_World")) (Math|Rotator|MakeRotator 0.0 9e+01 (.yaw (.rotation (Transformation|GetSocketTransform (Variables|Default|GetMesh) (select (Variables|Default|GetCannon%20Turn) "right_cannon" "left_cannon") "RTS_World")))) "1.000000,1.000000,1.000000") "AlwaysSpawn" 0 0))
  (Default|SetParams _returnvalue (/ (Transformation|GetDistanceTo (Game|Player|GetPlayerPawn 0)) 6.0)))

(fn PrepareSmashAttack
  (params (Delta%20Time :type Float%20%28double-precision%29))
  (bind _distance (CallFunction|GetDistancefromPlayer (Variables|Default|GetSmash%20Area)))
  (if (< _distance 5e+02)
    (Variables|Default|SetSmash%20Contemplation (- (Variables|Default|GetSmash%20Contemplation) Delta%20Time))
    (else
      (Variables|Default|SetSmash%20Contemplation 2.0))))

(fn Rotate
  (params (Delta :type Float%20%28double-precision%29))
  (Transformation|SetActorRotation (Math|Rotator|MakeRotator 0.0 0.0 (Math|Float|Lerp (.yaw (Transformation|GetActorRotation)) (.yaw (Math|Rotator|FindLookatRotation (Transformation|GetActorLocation) (Transformation|GetActorLocation (Game|Player|GetPlayerPawn 0)))) (* Delta (Variables|Default|GetRotation%20Speed))))))

(fn RollEyes
  (params (Delta :type Float%20%28double-precision%29))
  (bind _laser (Variables|Default|GetLaser))
  (Transformation|SetWorldRotation _laser (Math|Rotator|Lerp(Rotator) (Transformation|GetWorldRotation _laser) (Math|Rotator|FindLookatRotation (Transformation|GetWorldLocation (Variables|Default|GetLaser)) (+ (Transformation|GetActorLocation (Game|Player|GetPlayerPawn 0)) "0.000000,0.000000,-50.000000")) (* Delta 4.0) true) false false))