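; Test boss enemy with laser, missile and smash attacks, switched by events that first reset the others.
; Tick alternates the eye laser between a traced sweep and a recharging rewind, moving pre-placed VFX actors into view and back below ground.
; A looping timer, started on BeginPlay, fires missiles upward from alternating cannon sockets.
; The smash montage repeats while IsSmash is true, though nothing here sets it.
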(event Custom|SetSmashAnim
  ;[1 1 1] Comment
  (CallFunction|ResetBools)
  (if (Variables|Default|GetisSmash) :!label _label
    (Animation|Montage|PlayMontage (Variables|Default|GetMesh) 0 1.0 0.0 "Start"
      (:OnCompleted
        (Utilities|FlowControl|Delay 0.15)
        (goto _label)))))

(event Custom|ResetBools
  ;[1 1 1] Reset
  (Variables|Default|SetisSmash false)
  (Variables|Default|SetisLaser false)
  (Utilities|Time|PauseTimerbyHandle (Variables|Default|GetTimerM)))

(event Custom|SetLaserAnim
  ;[1 1 1] Comment
  (CallFunction|ResetBools)
  (Variables|Default|SetisLaser true))

(event Custom|SetMissileAnim
  ;[1 1 1] Comment
  (CallFunction|ResetBools)
  (Utilities|Time|UnpauseTimerbyHandle (Variables|Default|GetTimerM)))

(event EventBeginPlay
  (bind _returnvalue (Utilities|Time|SetTimerbyFunctionName 0 "Fire Missile" 1.0 true))
  (Variables|Default|SetTimerM _returnvalue)
  (bind _returnvalue_2 (Actor|GetActorOfClass "/Game/BossEnemy/VFX/BP_ImpactParticles.BP_ImpactParticles_C"))
  (Variables|Default|SetLaser%20Impact _returnvalue_2)
  (bind _returnvalue_3 (Actor|GetActorOfClass "/Game/BossEnemy/VFX/BP_PrepareLaser.BP_PrepareLaser_C"))
  (Variables|Default|SetLaser%20Prepare _returnvalue_3))

(event EventTick
  (params (DeltaSeconds :type Float%20%28single-precision%29))
  (bind _laser_impact (Variables|Default|GetLaser%20Impact))
  (bind _laser (Variables|Default|GetLaser))
  (bind _laser_prepare (Variables|Default|GetLaser%20Prepare))
  (bind _laser_2 (Variables|Default|GetLaser))
  (bind _returnvalue (Transformation|GetWorldLocation _laser))
  (bind _returnvalue_2 (Transformation|GetWorldRotation _laser_2))
  (if (Variables|Default|GetisLaser)
    (if (Variables|Default|GetisLaserTemp) :!label _label
      ;[1 1 1] Math
      (bind _output_get (Variables|Default|SetLaserTimer (- (Variables|Default|GetLaserTimer) DeltaSeconds)))
      (if (> _output_get 0.0)
        ;[1 1 1] Roll Eyes
        (Transformation|SetWorldRotation _laser_2 (Math|Rotator|MakeRotator (.roll _returnvalue_2) (.pitch _returnvalue_2) (+ (* 3e+01 DeltaSeconds) (.yaw _returnvalue_2))) false false)
        ;[1 1 1] VFX Laser
        (Components|Activation|Activate _laser false)
        (bind (_outhit _returnvalue_3) (Collision|LineTraceByChannel _returnvalue (+ _returnvalue (Math|Vector|RotateVector "2000.000000,0.000000,0.000000" (Transformation|GetWorldRotation _laser))) "TraceTypeQuery2" false 0 "ForOneFrame"))
        (if _returnvalue_3
          ;;[1 1 1] VFX Impact
          (Transformation|SetActorLocation _laser_impact (.Location (Collision|BreakHitResult _outhit)) false false)
          (Utilities|FlowControl|RetriggerableDelay 0.1)
          (Transformation|SetActorLocation _laser_impact "0.000000,0.000000,-200.000000" false false))
        (else
          (Variables|Default|SetisLaserTemp false)
          (goto _label)))
      (else
        ;[1 1 1] Math
        (bind _output_get_2 (Variables|Default|SetLaserTimer (+ (* DeltaSeconds 2.0) (Variables|Default|GetLaserTimer))))
        (if (<= _output_get_2 2.0)
          ;[1 1 1] Return Eyes
          (Transformation|SetWorldRotation _laser_2 (Math|Rotator|MakeRotator (.roll _returnvalue_2) (.pitch _returnvalue_2) (- (.yaw _returnvalue_2) (* DeltaSeconds 6e+01))) false false)
          ;[1 1 1] Charging VFX
          (Transformation|SetActorLocation _laser_prepare (Transformation|GetWorldLocation _laser_2) false false)
          (Utilities|FlowControl|Sequence
            (:then_0
              (Components|Activation|Deactivate _laser_2 :!label _label_2))
            (:then_1
              (Utilities|FlowControl|RetriggerableDelay 0.1)
              (Transformation|SetActorLocation _laser_prepare "0.000000,0.000000,-200.000000" false false)))
          (else
            (Variables|Default|SetisLaserTemp true)
            (goto _label)))))
    (else
      (goto _label_2))))

(fn ConstructionScript
  (bind _mesh (Variables|Default|GetMesh))
  (Transformation|AttachComponentToComponent (Variables|Default|GetL%20Hand%20Collider) _mesh "left_hand" "SnapToTarget" "SnapToTarget" "KeepRelative" true)
  (Transformation|AttachComponentToComponent (Variables|Default|GetR%20Hand%20Collider) _mesh "right_hand" "SnapToTarget" "SnapToTarget" "KeepRelative" true)
  (Transformation|AttachComponentToComponent (Variables|Default|GetLaser) _mesh "eye" "SnapToTarget" "SnapToTarget" "KeepRelative" true))

(fn FireMissile
  (Variables|Default|SetMissileTurn (not (Variables|Default|GetMissileTurn)))
  (bind _returnvalue (Game|SpawnActorfromClass "/Game/BossEnemy/BP_Missile.BP_Missile_C" (Math|Transform|MakeTransform (.location (Transformation|GetSocketTransform (Variables|Default|GetMesh) (select (Variables|Default|GetMissileTurn) "right_cannon" "left_cannon") "RTS_World")) (Math|Rotator|MakeRotator 0.0 9e+01 (.yaw (.rotation (Transformation|GetSocketTransform (Variables|Default|GetMesh) (select (Variables|Default|GetMissileTurn) "right_cannon" "left_cannon") "RTS_World")))) "1.000000,1.000000,1.000000") "AlwaysSpawn" 0 0))
  (Default|SetParams _returnvalue 1e+02))